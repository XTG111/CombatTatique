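; BP_LevelLoad is a level-loading Blueprint that switches between streaming sublevels by name, keeping track of the current one in LevelLoaded.
; LoadLevel unloads and hides the previous sublevel, then flags the requested one to load and become visible.
; It skips requests for the current level unless IsSame forces a reload, covering a default matching the initial map.
; The Square, Triangle, Hexagon test sequence and an alternative LoadLevelInstance call are unconnected.
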(event `self.ReceiveBeginPlay`)

(fn `LoadLevel`
  (params (Level :type String) (IsSame :type Boolean))
  (bind _returnvalue (`GameplayStatics.GetStreamingLevel` (`KismetStringLibrary.Conv_StringToName` (`self.LevelLoaded`))))
  (if (or IsSame (`KismetStringLibrary.NotEqual_StrStr` Level (`self.LevelLoaded`)))
    (`|ExecutionSequence`
      (:`then_0`
        ;[1 1 1] 加载下一个地图时，将上一个地图去掉
        (`/Engine/EditorBlueprintResources/StandardMacros.IsValid` _returnvalue
          (:`Is Valid`
            (set `LevelStreaming.bShouldBeLoaded` false _returnvalue)
            (set `LevelStreaming.bShouldBeVisible` false _returnvalue))))
      (:`then_1`
        (bind _output_get (set `self.LevelLoaded` Level))
        (bind _returnvalue_2 (`GameplayStatics.GetStreamingLevel` (`KismetStringLibrary.Conv_StringToName` _output_get)))
        ;[1 1 1] 两种Load Map的方法
        (`/Engine/EditorBlueprintResources/StandardMacros.IsValid` _returnvalue_2
          (:`Is Valid`
            (set `LevelStreaming.bShouldBeLoaded` true _returnvalue_2)
            (set `LevelStreaming.bShouldBeVisible` true _returnvalue_2)))))))

(fn `UserConstructionScript`)