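; BP_Actions_AddTile is a player action that adds a missing tile to the grid at a given index.
; ExecuteAction runs only when the index is not already valid in the grid instance held by PlayerAction.
; It ground-traces at that index's tile location, then calls AddGridTile with the traced location, the grid's rotation and scale, and a fixed tile type.
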(fn `ExecuteAction`
  (params (Index :type "IntPoint Structure"))
  (bind _index (`local.Index`))
  (bind _gridins (`/Game/Blueprints/Core/Player/BP_PlayerActions.GridIns` (`self.PlayerAction`)))
  (if (not (`/Game/Blueprints/Core/Grid/BP_Grid.Is Index Valid` (`/Game/Blueprints/Core/Player/BP_PlayerActions.GridIns` (`self.PlayerAction`)) (`local.Index`)))
    ;[1 1 1] 获取鼠标所在位置生成
    (bind (_tiletype _outlocation) (`/Game/Blueprints/Core/Grid/BP_Grid.TraceForGround` _gridins (`/Game/Blueprints/Core/Grid/BP_Grid.GetTileLocationFromGridIndex` _gridins _index)))
    (`/Game/Blueprints/Core/Grid/BP_Grid.AddGridTile` (`/Game/Blueprints/Core/Player/BP_PlayerActions.GridIns` (`self.PlayerAction`)) (make `/Game/Blueprints/Core/Grid/Utilities/S_TileData` (`local.Index`) "NewEnumerator1" (`KismetMathLibrary.MakeTransform` _outlocation (`/Game/Blueprints/Core/Grid/BP_Grid.GetTileRotateFromGridIndex` _gridins _index) (`/Game/Blueprints/Core/Grid/BP_Grid.GetTileScale` _gridins))))))

(fn `UserConstructionScript`
  (`parent.UserConstructionScript`))