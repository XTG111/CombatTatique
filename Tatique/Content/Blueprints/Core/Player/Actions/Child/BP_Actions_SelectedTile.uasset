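; Player action that selects a grid tile, toggling the selection when the same tile is targeted again.
; ExecuteAction moves a tile state from the previous SelecedTile to the new index through the player action's GridIns, or removes it and resets to a -999 sentinel on a repeat.
; On Destroyed, it runs ExecuteAction with that sentinel index to clear the current selection.
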(event `self.ReceiveDestroyed`
  (`self.ExecuteAction` (make `IntPoint` -999 -999)))

(fn `ExecuteAction`
  (params (Index :type "IntPoint Structure"))
  (bind _playeraction (`self.PlayerAction`))
  (bind _playeraction_2 (`self.PlayerAction`))
  (bind _playeraction_3 (`self.PlayerAction`))
  (if (!= (`/Game/Blueprints/Core/Player/BP_PlayerActions.SelecedTile` (`self.PlayerAction`)) (`local.Index`))
    ;[1 1 1] 删除之前选择的网格
    (`/Game/Blueprints/Core/Grid/BP_Grid.RemoveStateFromTile` (`/Game/Blueprints/Core/Player/BP_PlayerActions.GridIns` _playeraction) (`/Game/Blueprints/Core/Player/BP_PlayerActions.SelecedTile` _playeraction) "NewEnumerator2")
    (set `/Game/Blueprints/Core/Player/BP_PlayerActions.SelecedTile` (`local.Index`) (`self.PlayerAction`))
    (`/Game/Blueprints/Core/Grid/BP_Grid.AddStateToTile` (`/Game/Blueprints/Core/Player/BP_PlayerActions.GridIns` _playeraction_2) (`/Game/Blueprints/Core/Player/BP_PlayerActions.SelecedTile` _playeraction_2) "NewEnumerator2")
    (else
      (`/Game/Blueprints/Core/Grid/BP_Grid.RemoveStateFromTile` (`/Game/Blueprints/Core/Player/BP_PlayerActions.GridIns` _playeraction_3) (`/Game/Blueprints/Core/Player/BP_PlayerActions.SelecedTile` _playeraction_3) "NewEnumerator2")
      (set `/Game/Blueprints/Core/Player/BP_PlayerActions.SelecedTile` (make `IntPoint` -999 -999) (`self.PlayerAction`)))))

(fn `UserConstructionScript`
  (`parent.UserConstructionScript`))