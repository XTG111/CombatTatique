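; Player action Blueprint, a child in the actions hierarchy, that changes the type of a grid tile.
; ExecuteAction checks that the given index is valid on the grid referenced through PlayerAction, then looks up that tile's data.
; It calls AddGridTile with the same index, transform and states, substituting its TileType variable for the tile's type.
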(fn `ExecuteAction`
  (params (Index :type "IntPoint Structure"))
  (locals (Data :type "/Game/Blueprints/Core/Grid/Utilities/S_TileData Structure"))
  (bind (_data_index _data_type _data_transform _data_states) (break `/Game/Blueprints/Core/Grid/Utilities/S_TileData` (`local.Data`)))
  (if (`/Game/Blueprints/Core/Grid/BP_Grid.Is Index Valid` (`/Game/Blueprints/Core/Player/BP_PlayerActions.GridIns` (`self.PlayerAction`)) (`local.Index`))
    (set `local.Data` (`BlueprintMapLibrary.Map_Find` (`/Game/Blueprints/Core/Grid/BP_Grid.GridTiles` (`/Game/Blueprints/Core/Player/BP_PlayerActions.GridIns` (`self.PlayerAction`))) (`local.Index`)))
    (`/Game/Blueprints/Core/Grid/BP_Grid.AddGridTile` (`/Game/Blueprints/Core/Player/BP_PlayerActions.GridIns` (`self.PlayerAction`)) (make `/Game/Blueprints/Core/Grid/Utilities/S_TileData` _data_index (`self.TileType`) _data_transform _data_states))))

(fn `UserConstructionScript`
  (`parent.UserConstructionScript`))