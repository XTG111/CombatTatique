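; Player action that fills the grid pathfinding data with every tile's minimum cost to the currently selected tile.
; On execute, it runs the parent action, clears the previously generated pathfinding data and checks that the selected tile is valid.
; It then registers every grid tile as discovered with zero cost from start and its estimated minimum cost to that tile, honoring the Diagonals setting, without running a path search.
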(fn `ExecuteAction`
  (params (Index :type "IntPoint Structure"))
  (bind _playeraction (`self.PlayerAction`))
  (bind _playeraction_2 (`self.PlayerAction`))
  (bind _gridins (`/Game/Blueprints/Core/Player/BP_PlayerActions.GridIns` _playeraction_2))
  (`parent.ExecuteAction` Index)
  (`/Game/Blueprints/Core/Grid/BP_GridPathFindings.ClearGenerateData` (`/Game/Blueprints/Core/Grid/BP_Grid.GridPathFinding` (`/Game/Blueprints/Core/Player/BP_PlayerActions.GridIns` (`self.PlayerAction`))))
  (if (`/Game/Blueprints/Core/Grid/BP_Grid.Is Index Valid` (`/Game/Blueprints/Core/Player/BP_PlayerActions.GridIns` _playeraction) (`/Game/Blueprints/Core/Player/BP_PlayerActions.SelecedTile` _playeraction))
    (bind _keys (`BlueprintMapLibrary.Map_Keys` (`/Game/Blueprints/Core/Grid/BP_Grid.GridTiles` _gridins)))
    (for _array_element _keys
      (`/Game/Blueprints/Core/Grid/BP_GridPathFindings.DiscoverTile` (`/Game/Blueprints/Core/Grid/BP_Grid.GridPathFinding` (`/Game/Blueprints/Core/Player/BP_PlayerActions.GridIns` (`self.PlayerAction`))) (make `/Game/Blueprints/Core/Grid/Utilities/S_PathFindingData` _array_element 1 0 (`/Game/Blueprints/Core/Grid/BP_GridPathFindings.Get Minimum Cost Between Two Tiles` (`/Game/Blueprints/Core/Grid/BP_Grid.GridPathFinding` _gridins) _array_element (`/Game/Blueprints/Core/Player/BP_PlayerActions.SelecedTile` _playeraction_2) (`self.Diagonals`)))))))

(fn `UserConstructionScript`
  (`parent.UserConstructionScript`))