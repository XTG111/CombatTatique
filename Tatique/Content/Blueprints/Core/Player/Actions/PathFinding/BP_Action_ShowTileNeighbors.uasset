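; BP_Action_ShowTileNeighbors is a player action that marks the valid neighbors of a given grid tile.
; ExecuteAction clears one tile state from the grid, gets neighbors from GridPathFinding with optional diagonals, then adds that state to each.
; On Destroyed it runs again with an out-of-range index, which clears the marks left on the grid.
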(event `self.ReceiveDestroyed`
  (`self.ExecuteAction` (make `IntPoint` -999 -999)))

(fn `ExecuteAction`
  (params (Index :type "IntPoint Structure"))
  (`/Game/Blueprints/Core/Grid/BP_Grid.ClearStateFromTiles` (`/Game/Blueprints/Core/Player/BP_PlayerActions.GridIns` (`self.PlayerAction`)) "NewEnumerator3")
  (bind _neighbors (`/Game/Blueprints/Core/Grid/BP_GridPathFindings.GetValidTileNeighbor` (`/Game/Blueprints/Core/Grid/BP_Grid.GridPathFinding` (`/Game/Blueprints/Core/Player/BP_PlayerActions.GridIns` (`self.PlayerAction`))) Index (`self.Include Diagonals`)))
  (for _array_element _neighbors
    (`/Game/Blueprints/Core/Grid/BP_Grid.AddStateToTile` (`/Game/Blueprints/Core/Player/BP_PlayerActions.GridIns` (`self.PlayerAction`)) (break `/Game/Blueprints/Core/Grid/Utilities/S_PathFindingData` _array_element) "NewEnumerator3")))

(fn `UserConstructionScript`
  (`parent.UserConstructionScript`))