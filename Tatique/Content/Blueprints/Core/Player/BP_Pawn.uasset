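; BP_Pawn is a player pawn that serves as a camera rig with movement, stepped yaw rotation and spring-arm zoom.
; Axis inputs shift a desired location along the actor's forward and right vectors and adjust a clamped desired arm length, while button presses step the desired rotation.
; Tick smoothly interpolates location, rotation and arm length toward those targets, which BeginPlay seeds from the starting state.
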(event `self.ReceiveBeginPlay`
  ;[1 1 1] 开始时初始化缩放和视角位置
  (set `self.Location_Desired` (`self.K2_GetActorLocation`))
  (set `self.Zoom_Desired` (`SpringArmComponent.TargetArmLength` (`self.SpringArm`)))
  ;[1 1 1] 初始化旋转啊
  (set `self.Rotation_Desired` (`self.K2_GetActorRotation`)))

(event `self.ReceiveTick`
  (params (DeltaSeconds :type "Float (single-precision)"))
  (bind _springarm (`self.SpringArm`))
  (set `self.Delta Seconds` DeltaSeconds)
  (`|ExecutionSequence`
    (:`then_0`
      ;[1 1 1] tick 更新摄像机距离
      (set `SpringArmComponent.TargetArmLength` (`KismetMathLibrary.FInterpTo` (`SpringArmComponent.TargetArmLength` _springarm) (`self.Zoom_Desired`) (`self.Delta Seconds`) (`self.Zoom_Interp`)) _springarm))
    (:`then_1`
      ;[1 1 1] 左右前后移动
      (`self.K2_SetActorLocation` (`KismetMathLibrary.VInterpTo` (`self.K2_GetActorLocation`) (`self.Location_Desired`) (`self.Delta Seconds`) (`self.Location_Interp`))))
    (:`then_2`
      ;[1 1 1] 旋转视角
      (`self.K2_SetActorRotation` (`KismetMathLibrary.RInterpTo` (`self.K2_GetActorRotation`) (`self.Rotation_Desired`) (`self.Delta Seconds`) (`self.Rotation_Interp`))))))

(event `InputAxis|Zoom`
  (params (AxisValue :type "Float (single-precision)"))
  ;[1 1 1] 使用鼠标滚轮放大缩小
  (set `self.Zoom_Desired` (`KismetMathLibrary.FClamp` (+ (* AxisValue (* (`self.Zoom_Speed`) -1.0)) (`self.Zoom_Desired`)) (`self.Zoom_Min`) (`self.Zoom_Max`))))

(event `InputAxis|MoveForward`
  (params (AxisValue :type "Float (single-precision)"))
  ;[1 1 1] 前后移动视角
  (set `self.Location_Desired` (+ (`self.Location_Desired`) (* (`self.GetActorForwardVector`) (* AxisValue (`self.Location_Speed`))))))

(event `InputAxis|MoveRight`
  (params (AxisValue :type "Float (single-precision)"))
  ;[1 1 1] 左右移动视角
  (set `self.Location_Desired` (+ (`self.Location_Desired`) (* (`self.GetActorRightVector`) (* AxisValue (`self.Location_Speed`))))))

(event `InputAction|RotationRight`
  (params (Key :type "Key Structure"))
  ;[1 1 1] 控制旋转
  (:`Pressed`
    (set `self.Rotation_Desired` (`KismetMathLibrary.ComposeRotators` (`KismetMathLibrary.MakeRotator` 0.0 0.0 (* (`self.Rotation_Speed`) -1.0)) (`self.Rotation_Desired`)))))

(event `InputAction|RotationLeft`
  (params (Key :type "Key Structure"))
  ;[1 1 1] 控制旋转
  (:`Pressed`
    (set `self.Rotation_Desired` (`KismetMathLibrary.ComposeRotators` (`KismetMathLibrary.MakeRotator` 0.0 0.0 (`self.Rotation_Speed`)) (`self.Rotation_Desired`)))))

(fn `UserConstructionScript`)