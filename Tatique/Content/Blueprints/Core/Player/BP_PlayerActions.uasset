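; Player input actor for a tile grid that tracks the tile under the cursor and runs selected actions on it.
; Each tick it moves a state flag on BP_Grid from the previously hovered tile to the new one.
; Left and right mouse clicks execute their action actors on that tile.
; SetSelectedActions destroys and respawns those actors from given classes, passing itself in, then broadcasts the selection change.
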(event `self.ReceiveBeginPlay`
  (bind _returnvalue (`GameplayStatics.GetActorOfClass` "/Game/Blueprints/Core/Grid/BP_Grid.BP_Grid_C"))
  (set `self.GridIns` _returnvalue)
  (`self.EnableInput` (`GameplayStatics.GetPlayerController` 0)))

(event `self.ReceiveTick`
  (params (DeltaSeconds :type "Float (single-precision)"))
  (`self.UpdateHoveredTile`))

(event `Key|LeftMouseButton`
  (params (Key :type "Key Structure"))
  (:`Pressed`
    (`self.UpdateHoveredTile`)
    (`/Engine/EditorBlueprintResources/StandardMacros.IsValid` (`self.SelecetAction_LeftCheck`)
      (:`Is Valid`
        (`/Game/Blueprints/Core/Player/Actions/BP_Actions.ExecuteAction` (`self.SelecetAction_LeftCheck`) (`self.HoveredTile`))))))

(event `Key|RightMouseButton`
  (params (Key :type "Key Structure"))
  (:`Pressed`
    (`self.UpdateHoveredTile`)
    (`/Engine/EditorBlueprintResources/StandardMacros.IsValid` (`self.SelecetAction_RightCheck`)
      (:`Is Valid`
        (`/Game/Blueprints/Core/Player/Actions/BP_Actions.ExecuteAction` (`self.SelecetAction_RightCheck`) (`self.HoveredTile`))))))

(fn `SetSelectedActions`
  (params (LeftAction :type "/Game/Blueprints/Core/Player/Actions/BP_Actions Class Reference") (RightAction :type "/Game/Blueprints/Core/Player/Actions/BP_Actions Class Reference"))
  (bind _selecetaction_leftcheck (`self.SelecetAction_LeftCheck`))
  (bind _selecetaction_rightcheck (`self.SelecetAction_RightCheck`))
  (`|ExecutionSequence`
    (:`then_0`
      (`/Engine/EditorBlueprintResources/StandardMacros.IsValid` _selecetaction_leftcheck
        (:`Is Valid`
          (`self.K2_DestroyActor` _selecetaction_leftcheck)
          (set `self.SelecetAction_LeftCheck` null))
        (:`Is Not Valid`
          _))
      (if (`KismetSystemLibrary.IsValidClass` (`local.LeftAction`))
        (bind _returnvalue (`|SpawnActorFromClass` (`local.LeftAction`) (`KismetMathLibrary.MakeTransform` (0.0 0.0 0.0)) "AlwaysSpawn" "OverrideRootScale" null self null))
        (set `self.SelecetAction_LeftCheck` _returnvalue)))
    (:`then_1`
      (`/Engine/EditorBlueprintResources/StandardMacros.IsValid` _selecetaction_rightcheck
        (:`Is Valid`
          (`self.K2_DestroyActor` _selecetaction_rightcheck)
          (set `self.SelecetAction_RightCheck` null))
        (:`Is Not Valid`
          _))
      (if (`KismetSystemLibrary.IsValidClass` (`local.RightAction`))
        (bind _returnvalue_2 (`|SpawnActorFromClass` (`local.RightAction`) (`KismetMathLibrary.MakeTransform` (0.0 0.0 0.0)) "AlwaysSpawn" "OverrideRootScale" null self null))
        (set `self.SelecetAction_RightCheck` _returnvalue_2)))
    (:`then_2`
      (`self.OnSelectionActionChanged` (`self.SelecetAction_LeftCheck`) (`self.SelecetAction_RightCheck`)))))

(fn `UpdateHoveredTile`
  (bind _index (`/Game/Blueprints/Core/Grid/BP_Grid.GetTileIndexUnderCursor` (`self.GridIns`) 0))
  (if (!= _index (`self.HoveredTile`))
    (`/Game/Blueprints/Core/Grid/BP_Grid.ReMoveStateFromTile` (`self.GridIns`) (`self.HoveredTile`) "NewEnumerator1")
    (set `self.HoveredTile` _index)
    (`/Game/Blueprints/Core/Grid/BP_Grid.AddStateToTile` (`self.GridIns`) (`self.HoveredTile`) "NewEnumerator1")))

(fn `UserConstructionScript`)