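; A* pathfinder for the tile grid, finding a route between two tiles on square, triangle or hexagon layouts.
; FindPath expands the cheapest discovered tile through walkable neighbours within one tile height, then backtracks previous indices into a path.
; An insertion-sorted open list doubles estimated total cost and adds one for diagonal steps, favouring straight moves on ties.
; It runs instantly or with delayed iterations, broadcasting data updates for debug text and a completion event.
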(event `FindPathWithDelay`
  (if (> (`KismetArrayLibrary.Array_Length` (`self.DiscoveredTileIndexed`)) 0) :!label _label
    (bind _foundtargettile (`self.AnalyseNextDiscoveredTile`))
    (if _foundtargettile
      (bind _path (`self.GeneratePath`))
      (`self.OnPathFindingCompleted` _path)
      (else
        (`KismetSystemLibrary.RetriggerableDelay` (`self.DelayBetweenItterations`))
        (goto _label)))
    (else
      ;[1 1 1] 没有寻找到路径
      (`self.OnPathFindingCompleted` (`|MakeArray`)))))

(fn `AnalyseNextDiscoveredTile`
  (returns (FoundTargetTile :type Boolean))
  (bind _tilepathdata (`self.PullCheapestTileOutOfDiscoveredList`))
  (set `self.CurrentDiscoveredTile` _tilepathdata)
  ;[1 1 1] 计算邻接点数组
  (bind _neighbors (`self.GetValidTileNeighbor` (`.Index_2_DD755A07465A50D3F47D7386DD914686` (break `/Game/Blueprints/Core/Grid/Utilities/S_PathFindingData` (`self.CurrentDiscoveredTile`))) (`self.IncludeDiagonals`)))
  (set `self.CurrentNeighbors` _neighbors)
  (while (> (`KismetArrayLibrary.Array_Length` (`self.CurrentNeighbors`)) 0)
    ;[1 1 1] 统计邻接点消耗
    (bind _istargettile (`self.DiscoverNextNeighbor`))
    (if _istargettile
      (return true)))
  (return false))

(fn `ClearGenerateData`
  (`BlueprintMapLibrary.Map_Clear` (`self.PathFindingData`))
  (`KismetArrayLibrary.Array_Clear` (`self.DiscoveredTileSortingCosts`))
  (`KismetArrayLibrary.Array_Clear` (`self.DiscoveredTileIndexed`))
  (`KismetArrayLibrary.Array_Clear` (`self.AnalysedTileIndex`))
  ;[1 1 1] 广播，到DebugTextOnTiles
  (`self.OnPathFindingDataCleared`))

(fn `DiscoverNextNeighbor`
  (returns (IsTargetTile :type Boolean))
  (locals (CostFromStart :type Integer :default 0) (IndexInDiscovered :type Integer :default 0))
  (bind _indexindiscovered (`local.IndexInDiscovered`))
  (bind (_index _costtoentertile) (break `/Game/Blueprints/Core/Grid/Utilities/S_PathFindingData` (`self.CurrentNeighbor`)))
  (set `self.CurrentNeighbor` (`|GetArrayItem` (`self.CurrentNeighbors`)))
  (`KismetArrayLibrary.Array_Remove` (`self.CurrentNeighbors`))
  (if (not (`KismetArrayLibrary.Array_Contains` (`self.AnalysedTileIndex`) (`.Index_2_DD755A07465A50D3F47D7386DD914686` (break `/Game/Blueprints/Core/Grid/Utilities/S_PathFindingData` (`self.CurrentNeighbor`)))))
    (set `local.CostFromStart` (+ (`.CostFromStart_9_8635D7E1449233525146D29045DBE89D` (break `/Game/Blueprints/Core/Grid/Utilities/S_PathFindingData` (`self.CurrentDiscoveredTile`))) (`.CostToEnterTile_5_A1634F48483BC95606B16B9CD4C7ED13` (break `/Game/Blueprints/Core/Grid/Utilities/S_PathFindingData` (`self.CurrentNeighbor`)))))
    (bind _output_get (set `local.IndexInDiscovered` (`KismetArrayLibrary.Array_Find` (`self.DiscoveredTileIndexed`) (`.Index_2_DD755A07465A50D3F47D7386DD914686` (break `/Game/Blueprints/Core/Grid/Utilities/S_PathFindingData` (`self.CurrentNeighbor`))))))
    (if (not (== _output_get -1))
      (bind _output_get_2 (set `self.CurrentNeighbor` (`BlueprintMapLibrary.Map_Find` (`self.PathFindingData`) (`.Index_2_DD755A07465A50D3F47D7386DD914686` (break `/Game/Blueprints/Core/Grid/Utilities/S_PathFindingData` (`self.CurrentNeighbor`))))))
      (if (< (`local.CostFromStart`) (`.CostFromStart_9_8635D7E1449233525146D29045DBE89D` (break `/Game/Blueprints/Core/Grid/Utilities/S_PathFindingData` _output_get_2)))
        ;[1 1 1] 如果现在消耗小，则更新
        (`KismetArrayLibrary.Array_Remove` (`self.DiscoveredTileIndexed`) _indexindiscovered)
        (`KismetArrayLibrary.Array_Remove` (`self.DiscoveredTileSortingCosts`) _indexindiscovered)
        (else
          ;[1 1 1] 如果现在消耗大，则不处理
          (return false))))
    (`self.DiscoverTile` (make `/Game/Blueprints/Core/Grid/Utilities/S_PathFindingData` _index _costtoentertile (`local.CostFromStart`) (`self.Get Minimum Cost Between Two Tiles` _index (`self.TargetIndex`) (`self.IncludeDiagonals`)) (`.Index_2_DD755A07465A50D3F47D7386DD914686` (break `/Game/Blueprints/Core/Grid/Utilities/S_PathFindingData` (`self.CurrentDiscoveredTile`)))))
    ;[1 1 1] 判断邻接点是否时终点
    (if (`KismetMathLibrary.Equal_IntPointIntPoint` (`.Index_2_DD755A07465A50D3F47D7386DD914686` (break `/Game/Blueprints/Core/Grid/Utilities/S_PathFindingData` (`self.CurrentNeighbor`))) (`self.TargetIndex`))
      (return true)
      (else
        (return false)))
    (else
      (return false))))

(fn `DiscoverTile`
  (params (TilePathData :type "/Game/Blueprints/Core/Grid/Utilities/S_PathFindingData Structure"))
  (bind ((`Index_2_DD755A07465A50D3F47D7386DD914686` _index)) (break `/Game/Blueprints/Core/Grid/Utilities/S_PathFindingData` TilePathData))
  (`BlueprintMapLibrary.Map_Add` (`self.PathFindingData`) _index TilePathData)
  (`self.InsertTileInDiscoveredArray` (`local.TilePathData`))
  ;[1 1 1] 广播到DebugTextOnTiles
  (`self.OnPathFindingDataUpdated` _index))

(fn `FindPath`
  (params (start :type "IntPoint Structure") (target :type "IntPoint Structure") (Diagonals :type Boolean) (Delay :type "Float (double-precision)"))
  (returns (Path :type "Array of IntPoint Structure"))
  (bind _array (`|MakeArray` (struct) :!type "IntPoint Structure"))
  (bind _array_2 (`|MakeArray`))
  (set `self.StartIndex` start)
  (set `self.TargetIndex` target)
  (set `self.IncludeDiagonals` Diagonals)
  (set `self.DelayBetweenItterations` Delay)
  (`self.ClearGenerateData`)
  (bind _isvalid (`self.IsInputDataValid`))
  (if _isvalid
    (`self.DiscoverTile` (make `/Game/Blueprints/Core/Grid/Utilities/S_PathFindingData` (`self.StartIndex`) 1 0 (`self.Get Minimum Cost Between Two Tiles` (`self.StartIndex`) (`self.TargetIndex`) (`self.IncludeDiagonals`))))
    (if (<= (`self.DelayBetweenItterations`) 0.0)
      (while (> (`KismetArrayLibrary.Array_Length` (`self.DiscoveredTileIndexed`)) 0)
        (bind _foundtargettile (`self.AnalyseNextDiscoveredTile`))
        (if _foundtargettile
          (bind _path (`self.GeneratePath`))
          (`self.OnPathFindingCompleted` _path)
          (return _path)))
      ;[1 1 1] 没有寻找到路径
      (`self.OnPathFindingCompleted` _array_2)
      (return _array_2)
      (else
        (`self.FindPathWithDelay`)
        (return (`|MakeArray`))))
    (else
      ;[1 1 1] 如果输入无效则返回空
      (`self.OnPathFindingCompleted` _array)
      (return _array))))

(fn `GeneratePath`
  (returns (Path :type "Array of IntPoint Structure"))
  (locals (Current :type "IntPoint Structure") (InvertedPath :type "Array of IntPoint Structure") (Ret :type "Array of IntPoint Structure"))
  ;[1 1 1] 从终点退回起点生成
  (set `local.Current` (`self.TargetIndex`))
  (while (!= (`self.StartIndex`) (`local.Current`))
    ;[1 1 1] 存储结果数组，current每次根据之前存储的前一个Index回退
    (`KismetArrayLibrary.Array_Add` (`local.InvertedPath`) (`local.Current`))
    (set `local.Current` (`.PreviousIndex_12_BC31A124456A9DA8F279F0B82E6A9D8F` (break `/Game/Blueprints/Core/Grid/Utilities/S_PathFindingData` (`BlueprintMapLibrary.Map_Find` (`self.PathFindingData`) (`local.Current`))))))
  (bind (_arrayindex _arrayelement) (`/Engine/EditorBlueprintResources/StandardMacros.ReverseForEachLoop` (`local.InvertedPath`))
    (:`LoopBody`
      (`KismetArrayLibrary.Array_Add` (`local.Ret`) _arrayelement))
    (:`Completed`
      (return (`local.Ret`)))))

(fn `Get Minimum Cost Between Two Tiles`
  (params (Index1 :type "IntPoint Structure") (Index2 :type "IntPoint Structure") (Diagonals :type Boolean))
  (returns (MinCost :type Integer))
  (locals (x :type Integer :default 0) (y :type Integer :default 0))
  (bind _index2_x (break `IntPoint` (`local.Index2`)))
  (bind (_index1_x _index1_y) (break `IntPoint` (`local.Index1`)))
  (bind (_index1_x_2 _index1_y_2) (break `IntPoint` (`local.Index1`)))
  (bind _index2_x_2 (break `IntPoint` (`local.Index2`)))
  (bind _index1_x_3 (break `IntPoint` (`local.Index1`)))
  (bind _index1_x_4 (break `IntPoint` (`local.Index1`)))
  (bind (_returnvalue_x _returnvalue_y) (break `IntPoint` (- (`local.Index1`) (`local.Index2`))))
  (bind (_returnvalue_x_2 _returnvalue_y_2) (break `IntPoint` (- (`local.Index1`) (`local.Index2`))))
  (bind _returnvalue (<= (`local.x`) (`local.y`)))
  (bind _returnvalue_2 (< _index2_x_2 _index1_x_3))
  (bind (_returnvalue_x_3 _returnvalue_y_3) (break `IntPoint` (- (`local.Index1`) (`local.Index2`))))
  (bind (_returnvalue_x_4 _returnvalue_y_4) (break `IntPoint` (- (`local.Index1`) (`local.Index2`))))
  (bind (_returnvalue_x_5 _returnvalue_y_5) (break `IntPoint` (- (`local.Index1`) (`local.Index2`))))
  (bind _returnvalue_3 (* (`local.x`) 2))
  (bind _returnvalue_4 (`KismetMathLibrary.Abs_Int` _returnvalue_x))
  (bind _returnvalue_5 (<= (- (`local.x`) 1) (`local.y`)))
  (bind _returnvalue_6 (select `bool` (< _index2_x _index1_x_4) :`false` 1 :`true` -1))
  ;[1 1 1] 计算两个点之间的最少消耗移动数
  (switch `/Game/Blueprints/Core/Grid/GridShapes/E_GridShape` (`/Game/Blueprints/Core/Grid/BP_Grid.Shape` (`self.GridIns`))
    (:`NewEnumerator1`
      (if (`local.Diagonals`)
        ;;[1 1 1] 如果开启了对角线移动，等价于x,y之间差值的最大值
        (return (`KismetMathLibrary.Max` (`KismetMathLibrary.Abs_Int` _returnvalue_x_4) (`KismetMathLibrary.Abs_Int` _returnvalue_y_4)))
        (else
          ;;[1 1 1] 如果没有开启，那么就是x+y的值
          (return (+ (`KismetMathLibrary.Abs_Int` _returnvalue_x_3) (`KismetMathLibrary.Abs_Int` _returnvalue_y_3))))))
    (:`NewEnumerator2`
      (if (`local.Diagonals`)
        (return (+ (`KismetMathLibrary.Abs_Int` _returnvalue_x_2) (`KismetMathLibrary.Abs_Int` _returnvalue_y_2)))
        (else
          (set `local.x` (`KismetMathLibrary.Abs_Int` _returnvalue_x_5))
          (set `local.y` (`KismetMathLibrary.Abs_Int` _returnvalue_y_5))
          (if (select `bool` (== (`/Game/Blueprints/Core/Utilties/BLF_Utilties.IsIntEven` _index1_x) (`/Game/Blueprints/Core/Utilties/BLF_Utilties.IsIntEven` _index1_y)) :`false` (select `bool` _returnvalue_2 :`false` _returnvalue_5 :`true` _returnvalue) :`true` (select `bool` _returnvalue_2 :`false` _returnvalue :`true` _returnvalue_5))
            (return (+ (`local.x`) (`local.y`)))
            (elif (== (`/Game/Blueprints/Core/Utilties/BLF_Utilties.IsIntEven` (`local.x`)) (`/Game/Blueprints/Core/Utilties/BLF_Utilties.IsIntEven` (`local.y`)))
              (return _returnvalue_3)
              (else
                (return (+ _returnvalue_3 (select `bool` (== (`/Game/Blueprints/Core/Utilties/BLF_Utilties.IsIntEven` _index1_x_2) (`/Game/Blueprints/Core/Utilties/BLF_Utilties.IsIntEven` _index1_y_2)) :`false` (* _returnvalue_6 -1) :`true` _returnvalue_6)))))))))
    (:`NewEnumerator4`
      (return (+ _returnvalue_4 (`KismetMathLibrary.Max` (/ (- (`KismetMathLibrary.Abs_Int` _returnvalue_y) _returnvalue_4) 2)))))))

(fn `GetNeighborIndexes`
  (params (index :type "IntPoint Structure") (IncludeDiagonals :type Boolean))
  (returns (Neighbors :type "Array of IntPoint Structure"))
  (switch `/Game/Blueprints/Core/Grid/GridShapes/E_GridShape` (`/Game/Blueprints/Core/Grid/BP_Grid.Shape` (`self.GridIns`))
    (:`NewEnumerator1`
      (return (`self.GetNeighborIndexesForSquare` (`local.index`) (`local.IncludeDiagonals`))))
    (:`NewEnumerator2`
      (return (`self.GetNeighborIndexesForTriangle` (`local.index`) (`local.IncludeDiagonals`))))
    (:`NewEnumerator4`
      (return (`self.GetNeighborIndexesForHexagon` (`local.index`))))))

(fn `GetNeighborIndexesForHexagon`
  (params (index :type "IntPoint Structure"))
  (returns (Neighbors :type "Array of IntPoint Structure"))
  (locals (Ret :type "Array of IntPoint Structure"))
  (return (`|MakeArray` (+ (`local.index`) (make `IntPoint` 1 1)) (+ (`local.index`) (make `IntPoint` 0 2)) (+ (`local.index`) (make `IntPoint` -1 1)) (+ (`local.index`) (make `IntPoint` -1 -1)) (+ (`local.index`) (make `IntPoint` 0 -2)) (+ (`local.index`) (make `IntPoint` 1 -1)))))

(fn `GetNeighborIndexesForSquare`
  (params (index :type "IntPoint Structure") (IncludeDiagonals :type Boolean))
  (returns (Neighbors :type "Array of IntPoint Structure"))
  (locals (Ret :type "Array of IntPoint Structure"))
  (bind _array (`|MakeArray` (+ (`local.index`) (make `IntPoint` 1)) (+ (`local.index`) (make `IntPoint` -1)) (+ (`local.index`) (make `IntPoint` 0 1)) (+ (`local.index`) (make `IntPoint` 0 -1))))
  (if IncludeDiagonals
    (set `local.Ret` _array)
    (`KismetArrayLibrary.Array_Append` (`local.Ret`) (`|MakeArray` (+ (`local.index`) (make `IntPoint` 1 1)) (+ (`local.index`) (make `IntPoint` -1 -1)) (+ (`local.index`) (make `IntPoint` -1 1)) (+ (`local.index`) (make `IntPoint` 1 -1))))
    (return (`local.Ret`))
    (else
      (return _array))))

(fn `GetNeighborIndexesForTriangle`
  (params (index :type "IntPoint Structure") (IncludeDiagonals :type Boolean))
  (returns (Neighbors :type "Array of IntPoint Structure"))
  (locals (Ret :type "Array of IntPoint Structure"))
  (bind (_index_x _index_y) (break `IntPoint` (`local.index`)))
  (bind (_index_x_2 _index_y_2) (break `IntPoint` (`local.index`)))
  (set `local.Ret` (`|MakeArray` (+ (`local.index`) (make `IntPoint` 0 1)) (+ (`local.index`) (make `IntPoint` 0 -1))))
  (if (== (`/Game/Blueprints/Core/Utilties/BLF_Utilties.IsIntEven` _index_x_2) (`/Game/Blueprints/Core/Utilties/BLF_Utilties.IsIntEven` _index_y_2))
    (`KismetArrayLibrary.Array_Add` (`local.Ret`) (+ (`local.index`) (make `IntPoint` -1)))
    (else
      (`KismetArrayLibrary.Array_Add` (`local.Ret`) (+ (`local.index`) (make `IntPoint` 1)))))
  (if (`local.IncludeDiagonals`)
    (if (== (`/Game/Blueprints/Core/Utilties/BLF_Utilties.IsIntEven` _index_x) (`/Game/Blueprints/Core/Utilties/BLF_Utilties.IsIntEven` _index_y))
      (`KismetArrayLibrary.Array_Append` (`local.Ret`) (`|MakeArray` (+ (`local.index`) (make `IntPoint` 1)) (+ (`local.index`) (make `IntPoint` -1 -2)) (+ (`local.index`) (make `IntPoint` -1 2))))
      (else
        (`KismetArrayLibrary.Array_Append` (`local.Ret`) (`|MakeArray` (+ (`local.index`) (make `IntPoint` -1)) (+ (`local.index`) (make `IntPoint` 1 -2)) (+ (`local.index`) (make `IntPoint` 1 2))))))
    (return (`local.Ret`))
    (else
      (return (`local.Ret`)))))

(fn `GetTileSortingData`
  (params (TileData :type "/Game/Blueprints/Core/Grid/Utilities/S_PathFindingData Structure (by ref)"))
  (returns (Cost :type Integer))
  (bind ((`CostFromStart_9_8635D7E1449233525146D29045DBE89D` _costfromstart) (`MinimumCostToTarget_13_D2C327BF46089CA61829D7935867E237` _minimumcosttotarget)) (break `/Game/Blueprints/Core/Grid/Utilities/S_PathFindingData` TileData))
  (bind ((`Index_2_DD755A07465A50D3F47D7386DD914686` _index) (`PreviousIndex_12_BC31A124456A9DA8F279F0B82E6A9D8F` _previousindex)) (break `/Game/Blueprints/Core/Grid/Utilities/S_PathFindingData` TileData))
  (return (+ (* (+ _costfromstart _minimumcosttotarget) 2) (`KismetMathLibrary.Conv_BoolToInt` (`self.IsDiagonal` _index _previousindex)))))

(fn `GetValidTileNeighbor`
  (params (index :type "IntPoint Structure") (IncludeDiagonals :type Boolean))
  (returns (Neighbors :type "Array of /Game/Blueprints/Core/Grid/Utilities/S_PathFindingData Structure"))
  (locals (Data :type "/Game/Blueprints/Core/Grid/Utilities/S_TileData Structure") (`input data` :type "/Game/Blueprints/Core/Grid/Utilities/S_TileData Structure") (Ret :type "Array of /Game/Blueprints/Core/Grid/Utilities/S_PathFindingData Structure"))
  (bind _data_index (break `/Game/Blueprints/Core/Grid/Utilities/S_TileData` (`local.Data`)))
  (bind (_data_index_2 _data_type) (break `/Game/Blueprints/Core/Grid/Utilities/S_TileData` (`local.Data`)))
  (bind (_tile_size_x _tile_size_y _tile_size_z) (`KismetMathLibrary.BreakVector` (`/Game/Blueprints/Core/Grid/BP_Grid.Tile Size` (`self.GridIns`))))
  (set `local.input data` (`BlueprintMapLibrary.Map_Find` (`/Game/Blueprints/Core/Grid/BP_Grid.GridTiles` (`self.GridIns`)) (`local.index`)))
  (bind _neighbors (`self.GetNeighborIndexes` (`local.index`) (`local.IncludeDiagonals`)))
  (for _array_element _neighbors
    (set `local.Data` (`BlueprintMapLibrary.Map_Find` (`/Game/Blueprints/Core/Grid/BP_Grid.GridTiles` (`self.GridIns`)) _array_element))
    (if (`/Game/Blueprints/Core/Grid/Utilities/BFL_TileData.IsTileTypeWalkAble` _data_type)
      (if (<= (`KismetMathLibrary.Abs` (- (.z (.location (`.Transform_8_9C6A7C1C4635F658A66855A7D7345D6B` (break `/Game/Blueprints/Core/Grid/Utilities/S_TileData` (`local.Data`))))) (.z (.location (`.Transform_8_9C6A7C1C4635F658A66855A7D7345D6B` (break `/Game/Blueprints/Core/Grid/Utilities/S_TileData` (`local.input data`))))))) _tile_size_z)
        (`KismetArrayLibrary.Array_Add` (`local.Ret`) (make `/Game/Blueprints/Core/Grid/Utilities/S_PathFindingData` _data_index 1 999999 999999 (`local.index`))))))
  (return (`local.Ret`)))

(fn `InsertTileInDiscoveredArray`
  (params (TileData :type "/Game/Blueprints/Core/Grid/Utilities/S_PathFindingData Structure"))
  (locals (SortingData :type Integer :default 0))
  (bind _discoveredtilesortingcosts (`self.DiscoveredTileSortingCosts`))
  ;[1 1 1] 通过当前格子的数据，计算从起点经过该点到终点的消耗
  (set `local.SortingData` (`self.GetTileSortingData` TileData))
  (if (== (`KismetArrayLibrary.Array_Length` (`self.DiscoveredTileSortingCosts`)) 0)
    ;[1 1 1] 如果数组中没有数据，直接加入即可
    (`KismetArrayLibrary.Array_Add` (`self.DiscoveredTileSortingCosts`) (`local.SortingData`) :!label _label)
    (`KismetArrayLibrary.Array_Add` (`self.DiscoveredTileIndexed`) (`.Index_2_DD755A07465A50D3F47D7386DD914686` (break `/Game/Blueprints/Core/Grid/Utilities/S_PathFindingData` (`local.TileData`))))
    (elif (>= (`local.SortingData`) (`|GetArrayItem` _discoveredtilesortingcosts (`KismetArrayLibrary.Array_LastIndex` _discoveredtilesortingcosts)))
      (goto _label)
      (else
        ;[1 1 1] 如果有，就需要寻找数据的位置(升序插入排序)，然后插入数据
        (for (_array_element _array_index) (`self.DiscoveredTileSortingCosts`)
          (if (>= _array_element (`local.SortingData`))
            (`KismetArrayLibrary.Array_Insert` (`self.DiscoveredTileSortingCosts`) (`local.SortingData`) _array_index)
            (`KismetArrayLibrary.Array_Insert` (`self.DiscoveredTileIndexed`) (`.Index_2_DD755A07465A50D3F47D7386DD914686` (break `/Game/Blueprints/Core/Grid/Utilities/S_PathFindingData` (`local.TileData`))) _array_index)
            (break)))))))

(fn `IsDiagonal`
  (params (index1 :type "IntPoint Structure") (index2 :type "IntPoint Structure"))
  (returns (IsDiagonal :type Boolean))
  ;[1 1 1] 判断当前点是不是对角线点，通过Index1的由不包含对角线元素组成的数组，观测Index2
  (bind _neighbors (`self.GetNeighborIndexes` index1))
  (return (not (`KismetArrayLibrary.Array_Contains` _neighbors index2))))

(fn `IsInputDataValid`
  (returns (IsValid :type Boolean))
  ;[1 1 1] 判断输入的两个点是否有效
  (if (!= (`self.StartIndex`) (`self.TargetIndex`))
    (if (`/Game/Blueprints/Core/Grid/BP_Grid.IsTileWalkable` (`self.GridIns`) (`self.StartIndex`))
      (if (`/Game/Blueprints/Core/Grid/BP_Grid.IsTileWalkable` (`self.GridIns`) (`self.TargetIndex`))
        (return true)
        (else
          (return false)))
      (else
        (return false)))
    (else
      (return false))))

(fn `PullCheapestTileOutOfDiscoveredList`
  (returns (TilePathData :type "/Game/Blueprints/Core/Grid/Utilities/S_PathFindingData Structure"))
  (locals (TileIndex :type "IntPoint Structure"))
  (set `local.TileIndex` (`|GetArrayItem` (`self.DiscoveredTileIndexed`)))
  ;[1 1 1] 去掉已经计算了的节点
  (`KismetArrayLibrary.Array_Remove` (`self.DiscoveredTileIndexed`))
  (`KismetArrayLibrary.Array_Remove` (`self.DiscoveredTileSortingCosts`))
  ;[1 1 1] 向统计数组中加入该节点
  (`KismetArrayLibrary.Array_Add` (`self.AnalysedTileIndex`) (`local.TileIndex`))
  (return (`BlueprintMapLibrary.Map_Find` (`self.PathFindingData`) (`local.TileIndex`))))

(fn `UserConstructionScript`)